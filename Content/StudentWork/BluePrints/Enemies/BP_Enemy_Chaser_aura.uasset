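; Chaser enemy variant with an overlap aura that applies negative damage (-25) to the actor entering Sphere1.
; Begin overlap applies it and starts a looping timer with no event shown bound, though AuraDamage jumps to the same damage call.
; End overlap clears Health rather than the stored handle NewVar1.
; Move passes MyTarget as both pawn and goal to AIMoveTo; Attack only prints, and a spawn node is unwired.
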(event OnComponentBeginOverlap(Sphere1)
  (params (OverlappedComponent :type Primitive%20Component%20Object%20Reference) (OtherActor :type Actor%20Object%20Reference) (OtherComp :type Primitive%20Component%20Object%20Reference) (OtherBodyIndex :type Integer) (bFromSweep :type Boolean) (SweepResult :type Hit%20Result%20Structure%20%28by%20ref%29))
  (Utilities|FlowControl|Sequence
    (:then_0
      (bind _returnvalue (Utilities|Time|SetTimerbyEvent 0 1.0 true))
      (Variables|Default|SetNewVar_1 _returnvalue))
    (:then_1
      (Game|Damage|ApplyDamage OtherActor -25.0 0 0))))

(event OnComponentEndOverlap(Sphere1)
  (params (OverlappedComponent :type Primitive%20Component%20Object%20Reference) (OtherActor :type Actor%20Object%20Reference) (OtherComp :type Primitive%20Component%20Object%20Reference) (OtherBodyIndex :type Integer))
  ;[1 1 1] On End overlap,Clear the timer
  (Utilities|Time|ClearandInvalidateTimerbyHandle (Variables|Default|GetHealth)))

(event Custom|AuraDamage
  (Game|Damage|ApplyDamage (stale OnComponentBeginOverlap(Sphere1) OtherActor) -25.0 0 0))

(event EventMove
  (bind _mytarget (Variables|Default|GetMyTarget))
  (Utilities|IsValid _mytarget
    (:Is%20Valid
      (AI|AIMoveTo (Variables|Default|GetMyTarget) "0, 0, 0" _mytarget 5.0 false))))

(event EventAttack
  (Development|PrintString "enemy attack"))

(fn ConstructionScript
  (|CallParentFunction))