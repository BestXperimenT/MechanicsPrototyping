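; Boss enemy Blueprint that chases a target and fires random projectiles.
; BeginPlay fills its health to a boss-sized maximum, and the Move event uses AI MoveTo toward MyTarget when valid.
; Attack spawns a Projectiles array class at FireArrow's transform and prints debug text.
; The random index includes the array length, so can overrun, and is re-rolled separately for storing, spawning and printing.
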(event EventBeginPlay
  ;[1 1 1] Health event
  (bind _output_get (Variables|Default|SetMaxHealth 2e+03))
  (Variables|Default|SetCurrentHealth _output_get))

(event EventMove
  (bind _mytarget (Variables|Default|GetMyTarget))
  ;[1 1 1] Move event
  (Utilities|IsValid _mytarget
    (:Is%20Valid
      (AI|AIMoveTo self "0, 0, 0" _mytarget 5.0 false))))

(event EventAttack
  (bind _projectiles (Variables|Default|GetProjectiles))
  (bind _firearrow (Variables|Default|GetFireArrow))
  (bind _returnvalue (Utilities|Array|Length _projectiles))
  (bind _returnvalue_2 (Math|Random|RandomIntegerinRange 0 _returnvalue))
  ;[1 1 1] Attack event
  (Development|PrintString "enemy attack")
  (Variables|Default|SetProjectile%20Index _returnvalue_2)
  (Game|SpawnActorfromClass (Utilities|Array|Get(acopy) _projectiles _returnvalue_2) (Math|Transform|MakeTransform (Transformation|GetWorldLocation _firearrow) (Transformation|GetWorldRotation _firearrow) "1.000000,1.000000,1.000000") "Undefined" "MultiplyWithRoot" 0 0)
  (Development|PrintString (Utilities|String|ToString(Integer) _returnvalue_2)))

(fn ConstructionScript
  (|CallParentFunction))