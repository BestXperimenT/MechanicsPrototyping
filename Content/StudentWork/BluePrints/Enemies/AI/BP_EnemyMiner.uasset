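; BP_EnemyMiner is an enemy AI character that patrols and deploys mines.
; Attack waits briefly, then spawns a BP_WorldMine at its FireArrow's location and rotation.
; TankPatrol slows walk speed and uses AIMoveTo through eight indexed PatrolLocation points, pausing randomly after each successful move.
; The patrol re-calls itself before advancing the wrapping index, and has no handling for failed moves.
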(event Custom|TankPatrol
  ;[1 1 1] TankPatrol
  (Variables|/Script/Engine.CharacterMovementComponent|SetMaxWalkSpeed (Variables|Character|GetCharacterMovement) 1.5e+02)
  (AI|AIMoveTo self (Utilities|Array|Get(acopy) (Variables|Default|GetPatrolLocation) (Variables|Default|GetLocations)) 0 5.0 false
    (:then
      (Utilities|FlowControl|Delay (Math|Random|RandomFloatinRange 1.0 3.0))
      (CallFunction|TankPatrol)
      (Math|Integer|IncrementInt (Variables|Default|GetLocations)
        (:%20%20
          (if (== (Variables|Default|GetLocations) 8)
            (Variables|Default|SetLocations 0)))))))

(event EventAttack
  (bind _firearrow (Variables|Default|GetFireArrow))
  ;[1 1 1] Attack
  (Utilities|FlowControl|Delay 2.0)
  (Game|SpawnActorfromClass "/Game/StudentWork/BluePrints/Mine/BP_WorldMine.BP_WorldMine_C" (Math|Transform|MakeTransform (Transformation|GetWorldLocation _firearrow) (Transformation|GetWorldRotation _firearrow) "1.000000,1.000000,1.000000") "Undefined" "MultiplyWithRoot" 0 0))

(fn ConstructionScript
  (|CallParentFunction))