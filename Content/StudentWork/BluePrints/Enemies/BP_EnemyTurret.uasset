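; BP_EnemyTurret is an enemy turret that fires on a fixed interval and can be destroyed by damage.
; On BeginPlay it sets its health and starts a looping timer that calls FireProjectile, which spawns an actor at the Arrow component's location and rotation.
; AnyDamage subtracts from current health and destroys the turret once it reaches zero or below.
; The graph has no targeting or aiming logic.
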(event Custom|FireProjectile
  (bind _arrow (Variables|Default|GetArrow))
  (Game|SpawnActorfromClass "/Game/StudentWork/Projectiles/BP_EnemyProjectile.BP_EnemyProjectile_C" (Math|Transform|MakeTransform (Transformation|GetWorldLocation _arrow) (Transformation|GetWorldRotation _arrow) "1.000000,1.000000,1.000000") "Undefined" "MultiplyWithRoot" 0 0))

(event EventBeginPlay
  (bind _output_get (Variables|Default|SetMaxhealth 6e+01))
  (Variables|Default|SetCurrentHealth _output_get)
  (bind _returnvalue (Utilities|Time|SetTimerbyEvent (delegate Custom|FireProjectile) 1.0 true))
  (Variables|Default|SetFireTimer _returnvalue))

(event Game|Damage|EventAnyDamage
  (params (Damage :type Float%20%28single-precision%29) (DamageType :type Damage%20Type%20Object%20Reference) (InstigatedBy :type Controller%20Object%20Reference) (DamageCauser :type Actor%20Object%20Reference))
  (Variables|Default|SetCurrentHealth (- (Variables|Default|GetCurrentHealth) Damage))
  (if (<= (Variables|Default|GetCurrentHealth) 0.0)
    (Actor|DestroyActor)))

(fn ConstructionScript)