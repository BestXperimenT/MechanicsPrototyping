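; BP_EnemyMiner is an enemy Blueprint that chases a target and lays mines in the world.
; Its Move event sends the pawn toward MyTarget with AI MoveTo when that target is valid.
; Its Attack event waits through a short delay, then spawns a BP_WorldMine at the FireArrow component's location and rotation.
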(event EventMove
  (bind _mytarget (Variables|Default|GetMyTarget))
  ;[1 1 1] AI Move
  (Utilities|IsValid _mytarget
    (:Is%20Valid
      (AI|AIMoveTo self "0, 0, 0" _mytarget 5.0 false))))

(event EventAttack
  (bind _firearrow (Variables|Default|GetFireArrow))
  ;[1 1 1] Attack
  (Utilities|FlowControl|Delay 2.0)
  (Game|SpawnActorfromClass "/Game/StudentWork/BluePrints/Mine/BP_WorldMine.BP_WorldMine_C" (Math|Transform|MakeTransform (Transformation|GetWorldLocation _firearrow) (Transformation|GetWorldRotation _firearrow) "1.000000,1.000000,1.000000") "Undefined" "MultiplyWithRoot" 0 0))

(fn ConstructionScript
  (|CallParentFunction))