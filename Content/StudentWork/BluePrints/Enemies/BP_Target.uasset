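; BP_Target is an explosive barrel that detonates after taking any damage.
; The first hit, gated by DoOnce, sets the flash material and plays a timeline that drives its scalar parameter.
; When the timeline finishes, a debug-drawn multi-sphere trace applies flat damage to each hit actor, then a Niagara bang spawns and the barrel is destroyed.
; The construction script creates a dynamic flash material instance on the barrel.
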(event Game|Damage|EventAnyDamage
  (params (Damage :type Float%20%28single-precision%29) (DamageType :type Damage%20Type%20Object%20Reference) (InstigatedBy :type Controller%20Object%20Reference) (DamageCauser :type Actor%20Object%20Reference))
  (bind _returnvalue (Transformation|GetActorLocation))
  (bind _barrel (Variables|Default|GetBarrel))
  (Utilities|FlowControl|DoOnce false
    (:Completed
      (Rendering|Material|SetMaterial _barrel 0 "/Game/StudentWork/MyMaterials/Flash_Barrel.Flash_Barrel")
      (bind _flash (Timeline|Flash Play)
        (:Update
          (Rendering|Material|SetScalarParameterValueonMaterials _barrel "Flash_Barrel" _flash))
        (:Finished
          (bind _outhits (Collision|MultiSphereTraceForObjects _returnvalue _returnvalue 3e+02 (Variables|Default|GetObject%20Types) false 0 "ForDuration" false))
          (for _array_element _outhits
            (Game|Damage|ApplyDamage (.HitActor (Collision|BreakHitResult _array_element)) 3e+01 0 0))
          (Niagara|SpawnSystematLocation "/Game/StudentWork/Particles/NS_Bang.NS_Bang" (Transformation|GetActorLocation))
          (Actor|DestroyActor))))))

(fn ConstructionScript
  (bind _returnvalue (Rendering|Material|CreateDynamicMaterialInstance (Variables|Default|GetBarrel) 0 "/Game/StudentWork/MyMaterials/Flash_Barrel.Flash_Barrel" "None" :!class /Script/Engine.PrimitiveComponent))
  (LocalVariables|SetFlash%20Material _returnvalue))