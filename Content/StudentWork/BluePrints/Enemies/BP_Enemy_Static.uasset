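; BP_Enemy_Static is an enemy Blueprint whose attack fires homing missiles at its target.
; The Attack event spawns a BP_Enemy_HomingMissile at the FireArrow component, with a random direction inside a narrow cone around the arrow's forward vector.
; After a validity check, it sets the missile's ProjectileMovement homing target to MyTarget's capsule component.
; The construction script only calls its parent.
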(event EventAttack
  (bind _firearrow (Variables|Default|GetFireArrow))
  (bind _returnvalue (Game|SpawnActorfromClass "/Game/StudentWork/Projectiles/BP_Enemy_HomingMissile.BP_Enemy_HomingMissile_C" (Math|Transform|MakeTransform (Transformation|GetWorldLocation _firearrow) (Math|Conversions|RotationFromXVector (Math|Random|RandomUnitVectorinConeinDegrees (Math|Rotator|GetRotationXVector (Transformation|GetWorldRotation _firearrow)) 5.0)) "1.000000,1.000000,1.000000") "Undefined" "MultiplyWithRoot" 0 0))
  (Utilities|IsValid 0
    (:Is%20Valid
      (Variables|/Script/Engine.ProjectileMovementComponent|SetHomingTargetComponent (Variables|/Game/StudentWork/Projectiles/BP_Enemy_HomingMissile.BP_Enemy_HomingMissile_C|GetProjectileMovement _returnvalue) (Variables|/Script/Engine.Character|GetCapsuleComponent (Variables|Default|GetMyTarget))))))

(fn ConstructionScript
  (|CallParentFunction))