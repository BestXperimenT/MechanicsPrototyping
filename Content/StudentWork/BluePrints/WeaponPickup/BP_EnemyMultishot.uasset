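; BP_EnemyMultishot is a weapon Blueprint that fires a fanned volley of projectiles from a tank, apparently for enemies.
; When triggered off cooldown, it spawns ProjectileCount BP_Multifire actors at the tank's DirectionArrow.
; Each shot takes the arrow's rotation with a yaw offset, plus a Spread rotation scaled by its index.
; Firing sets a cooldown flag, which a looping timer, set inside the spawn loop, clears.
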(event Custom|End%20Cooldown
  (Variables|Default|Setcooldown false))

(event EventTriggered
  (bind _mytank (Variables|Default|GetMyTank))
  (bind _directionarrow (Variables|/Game/Blueprints/BP_PlayerCharacter.BP_PlayerCharacter_C|GetDirectionArrow _mytank))
  (bind _returnvalue (Transformation|GetWorldRotation _directionarrow))
  (bind (_roll _pitch _yaw) (Math|Rotator|BreakRotator _returnvalue))
  (if (not (Variables|Default|GetCooldown))
    (for _index (range 1 (Variables|Default|GetProjectileCount))
      (Game|SpawnActorfromClass "/Game/StudentWork/Projectiles/BP_Multifire.BP_Multifire_C" (Math|Transform|MakeTransform (Transformation|GetWorldLocation (Variables|/Game/Blueprints/BP_PlayerCharacter.BP_PlayerCharacter_C|GetDirectionArrow _mytank)) (Math|Rotator|CombineRotators (Math|Rotator|MakeRotator _roll _pitch (+ _yaw (Variables|Default|GetRotationOffset))) (* (Math|Rotator|MakeRotator 0.0 0.0 (Variables|Default|GetSpread)) _index)) "1.000000,1.000000,1.000000") "Undefined" "MultiplyWithRoot" 0 0)
      (Variables|Default|Setcooldown true)
      (Utilities|Time|SetTimerbyEvent (delegate Custom|End%20Cooldown) 0.4 true))))

(fn ConstructionScript
  (|CallParentFunction))