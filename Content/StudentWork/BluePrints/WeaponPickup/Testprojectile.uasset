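; Testprojectile is a projectile actor that deals damage to whatever its collision sphere hits, then destroys itself.
; Its construction script copies exposed speed variables into the ProjectileMovement component.
; It also derives the Niagara effect's Size parameter and the sphere's collision radius from MaxSpeed, so faster projectiles appear and collide larger.
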(event OnComponentHit(Sphere)
  (params (HitComponent :type Primitive%20Component%20Object%20Reference) (OtherActor :type Actor%20Object%20Reference) (OtherComp :type Primitive%20Component%20Object%20Reference) (NormalImpulse :type Vector :default "0, 0, 0") (Hit :type Hit%20Result%20Structure%20%28by%20ref%29))
  ;[1 1 1] Damage Event
  (Game|Damage|ApplyDamage OtherActor 1e+01 0 0)
  (Actor|DestroyActor))

(fn ConstructionScript
  (bind _projectilemovement (Variables|Default|GetProjectileMovement))
  (bind _max_speed (Variables|Default|GetMax%20Speed))
  (bind _returnvalue (/ _max_speed 1e+02))
  (Variables|/Script/Engine.ProjectileMovementComponent|SetInitialSpeed _projectilemovement (Variables|Default|GetInitial%20Speed))
  (Variables|/Script/Engine.ProjectileMovementComponent|SetMaxSpeed _projectilemovement (Variables|Default|GetMax%20Speed))
  (Effects|Components|ParticleSystem|SetFloatParameter (Variables|Default|GetNiagara) "Size" _returnvalue)
  (Components|Sphere|SetSphereRadius (Variables|Default|GetSphere) _returnvalue true))