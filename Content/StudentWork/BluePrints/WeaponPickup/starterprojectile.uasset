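; Starter projectile Blueprint with a Niagara effect that scales with a charge value.
; The construction script copies the InitialSpeed and MaxSpeed variables into the ProjectileMovement component.
; A Chargesize event divides the incoming ChargeSize by 100, prints it to the log and sets it as the Niagara Size parameter.
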(event Custom|Charge%20size
  (params (Charge%20Size :type Float%20%28double-precision%29))
  (bind _returnvalue (/ Charge%20Size 1e+02))
  ;[1 1 1] Niagra charge effect
  (Development|PrintString (Utilities|String|ToString(Float) _returnvalue) false)
  (Effects|Components|ParticleSystem|SetFloatParameter (Variables|Default|GetNiagara) "Size" _returnvalue))

(event EventBeginPlay)

(fn ConstructionScript
  (bind _projectilemovement (Variables|Default|GetProjectileMovement))
  ;[1 1 1] Projectile Movement
  (Variables|/Script/Engine.ProjectileMovementComponent|SetInitialSpeed _projectilemovement (Variables|Default|GetInitial%20Speed))
  (Variables|/Script/Engine.ProjectileMovementComponent|SetMaxSpeed _projectilemovement (Variables|Default|GetMax%20Speed)))